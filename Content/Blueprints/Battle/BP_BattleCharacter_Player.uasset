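; Player-controlled battle character Blueprint that extends a parent character with an in-world actions widget.
; On BeginPlay it registers itself as the battle controller's ActualChara and initialises the WBP_CharaActions skill selector with its SkillsList.
; Each tick it billboards the widget component toward the player battle camera using a look-at rotation.
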(event `self.ReceiveBeginPlay`
  (`parent.ReceiveBeginPlay`)
  (set `/Game/Blueprints/Battle/BP_BattlePlayerController.ActualChara` self (`/Game/Blueprints/Battle/BP_FL_Getters.GetBattleController`))
  (bind _aswbp_chara_actions (cast `/Game/UI/Battle/WBP_CharaActions` (`WidgetComponent.GetWidget` (`self.Widget`))))
  (`/Game/UI/Battle/WBP_SkillsSelect.Initialisation` (`/Game/UI/Battle/WBP_CharaActions.WBP_SkillsSelect` _aswbp_chara_actions) (`self.SkillsList`)))

(event `self.ReceiveTick`
  (params (DeltaSeconds :type "Float (single-precision)"))
  (`parent.ReceiveTick` DeltaSeconds)
  (`SceneComponent.K2_SetWorldRotation` (`self.Widget`) (`KismetMathLibrary.FindLookAtRotation` (`SceneComponent.K2_GetComponentLocation` (`self.Widget`)) (`self.K2_GetActorLocation` (`/Game/Blueprints/Battle/BP_FL_Getters.GetPlayerBattleCamera`))) false false))

(fn `UserConstructionScript`
  (`parent.UserConstructionScript`))