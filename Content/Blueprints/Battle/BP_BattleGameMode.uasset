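; Game mode for battles that runs the turn cycle between the player and a list of enemies.
; Shortly after BeginPlay it hands the turn to the battle controller's StartTurn.
; On the enemies' turn it plays a UI banner animation, then has each enemy attack in sequence, waiting each attack's returned duration before returning control to the player.
; Helpers expose a random enemy and the controller's current character.
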(event `self.ReceiveBeginPlay`
  (`KismetSystemLibrary.Delay` 0.2)
  (`self.PlayerTurn`))

(event `EnemiesTurn`
  (bind _battleui (`/Game/Blueprints/Battle/BP_BattlePlayerController.BattleUI` (`/Game/Blueprints/Battle/BP_FL_Getters.GetBattleController`)))
  (bind _ennemiesturn (`/Game/UI/Battle/WBP_BattleUI.EnnemiesTurn` _battleui))
  (`UserWidget.PlayAnimation` _battleui _ennemiesturn 0.0 1 "Forward" 1.0 false)
  (`KismetSystemLibrary.Delay` (`WidgetAnimation.GetEndTime` _ennemiesturn))
  (set `self.Index` 0)
  (bind _animationlenght (`/Game/Blueprints/Battle/BP_BattleCharacter_Ennemy.Attack` (`|GetArrayItem` (`self.Ennemies`) (`self.Index`)) :!label _label))
  (`KismetSystemLibrary.Delay` _animationlenght)
  (bind _result (`/Engine/EditorBlueprintResources/StandardMacros.IncrementInt` (`self.Index`))
    (:`  `
      (if (>= _result (`KismetArrayLibrary.Array_Length` (`self.Ennemies`)))
        (`self.PlayerTurn`)
        (else
          (goto _label))))))

(fn `GetPlayerCharacter`
  (returns (ActualChara :type "/Game/Blueprints/Battle/BP_BattleCharacter_Player Object Reference"))
  (return (`/Game/Blueprints/Battle/BP_BattlePlayerController.ActualChara` (`/Game/Blueprints/Battle/BP_FL_Getters.GetBattleController`))))

(fn `PlayerTurn`
  (`/Game/Blueprints/Battle/BP_BattlePlayerController.StartTurn` (`/Game/Blueprints/Battle/BP_FL_Getters.GetBattleController`)))

(fn `SelectEnnemy`
  (returns (OutItem :type "/Game/Blueprints/Battle/BP_BattleCharacter_Ennemy Object Reference"))
  (return (`KismetArrayLibrary.Array_Random` (`self.Ennemies`))))

(fn `UserConstructionScript`)