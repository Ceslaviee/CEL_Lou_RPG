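; BP_BattleCharacter is a battle character Blueprint that tracks hit points and reflects them in a battle UI.
; ChangeHP stores the new value without clamping, sends the HP/HPMax ratio to CharacterBattleUI, and calls OnDeath at zero or below.
; AddHP applies a relative change through ChangeHP.
; OnDeath is a placeholder that prints a debug string, and the event graph holds no active logic.
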(fn `AddHP`
  (params (B :type "Float (double-precision)"))
  (`self.ChangeHP` (+ (`self.HP`) B)))

(fn `ChangeHP`
  (params (HP :type "Float (double-precision)"))
  (bind _output_get (set `self.HP` HP))
  (`/Game/UI/Battle/WBP_CharacterBattleUI.UpdateHP` (`self.Character Battle UI`) (/ _output_get (`self.HPMax`)))
  (if (<= (`self.HP`) 0.0)
    (`self.OnDeath`)))

(fn `OnDeath`
  (`KismetSystemLibrary.PrintString` "OnoImDead"))

(fn `UserConstructionScript`)