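; Blueprint function library of getters for core battle-mode framework objects.
; It provides the player battle camera pawn, the battle player controller and the battle game mode.
; Each getter casts the engine's player zero pawn, player zero controller or current game mode to its battle Blueprint class and returns it.
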(fn `GetBattleController`
  (returns (`AsBP Battle Player Controller` :type "/Game/Blueprints/Battle/BP_BattlePlayerController Object Reference"))
  (bind _asbp_battle_player_controller (cast `/Game/Blueprints/Battle/BP_BattlePlayerController` (`GameplayStatics.GetPlayerController` null)))
  (return _asbp_battle_player_controller))

(fn `GetBattleGameMode`
  (returns (`AsBP Battle Game Mode` :type "/Game/Blueprints/Battle/BP_BattleGameMode Object Reference"))
  (bind _asbp_battle_game_mode (cast `/Game/Blueprints/Battle/BP_BattleGameMode` (`GameplayStatics.GetGameMode` null)))
  (return _asbp_battle_game_mode))

(fn `GetPlayerBattleCamera`
  (returns (`AsBP Player Battle Camera` :type "/Game/Blueprints/Battle/BP_PlayerBattleCamera Object Reference"))
  (bind _asbp_player_battle_camera (cast `/Game/Blueprints/Battle/BP_PlayerBattleCamera` (`GameplayStatics.GetPlayerPawn` null)))
  (return _asbp_player_battle_camera))