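; BP_Skills is a skill Blueprint that applies an action to targets chosen by its Target setting.
; LaunchAction switches on Target and uses the GameMode to resolve the player character, one selected enemy or every enemy in its Ennemies list.
; It calls Action on each resolved target; Action is empty here, leaving the actual effect undefined in this asset.
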(fn `Action`
  (params (Target :type "/Game/Blueprints/Battle/BP_BattleCharacter Object Reference")))

(fn `LaunchAction`
  (params (GameMode :type "/Game/Blueprints/Battle/BP_BattleGameMode Object Reference"))
  (switch `/Game/Blueprints/Enums/ENUM_Targets` (`self.Target`)
    (:`NewEnumerator0`
      (`self.Action` (`/Game/Blueprints/Battle/BP_BattleGameMode.GetPlayerCharacter` (`local.GameMode`))))
    (:`NewEnumerator1`
      (bind _outitem (`/Game/Blueprints/Battle/BP_BattleGameMode.SelectEnnemy` (`local.GameMode`)))
      (`self.Action` _outitem))
    (:`NewEnumerator2`
      (for _array_element (`/Game/Blueprints/Battle/BP_BattleGameMode.Ennemies` (`local.GameMode`))
        (`self.Action` _array_element)))))